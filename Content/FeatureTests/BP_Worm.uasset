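; BP_Worm is a feature test actor that drives a three-segment worm (Head, Middle, Tail) in an undulating motion using Physics Control.
; On BeginPlay it creates named parent-space controls linking Head to Middle and Middle to Tail.
; Each Tick sets both controls' target pitch from GetMovement, a time-based sine wave with a quarter-cycle phase offset between the joints, producing a travelling wave.
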(event EventBeginPlay
  (bind _physicscontrol (Variables|Default|GetPhysicsControl))
  (Class|PhysicsControlComponent|MakeNamedControl :self _physicscontrol :Name "HeadMiddle" :ParentMeshComponent (Variables|Default|GetHead) :ChildMeshComponent (Variables|Default|GetMiddle) :ControlData (Variables|Default|GetParentSpaceControlData))
  (Class|PhysicsControlComponent|MakeNamedControl :self _physicscontrol :Name "MiddleTail" :ParentMeshComponent (Variables|Default|GetMiddle) :ChildMeshComponent (Variables|Default|GetTail) :ControlData (Variables|Default|GetParentSpaceControlData)))

(event Collision|EventActorBeginOverlap
  (params (OtherActor :type Actor%20Object%20Reference)))

(event EventTick
  (params (DeltaSeconds :type Float%20%28single-precision%29))
  (Class|PhysicsControlComponent|SetControlTargetOrientation (Variables|Default|GetPhysicsControl) "HeadMiddle" (Math|Rotator|MakeRotator 0.0 (CallFunction|GetMovement 0.0) 0.0) 0.0 true false)
  (Class|PhysicsControlComponent|SetControlTargetOrientation (Variables|Default|GetPhysicsControl) "MIddleTail" (Math|Rotator|MakeRotator 0.0 (CallFunction|GetMovement 9e+01) 0.0) 0.0 true false))

(fn ConstructionScript)

(fn GetMovement
  (params (Offset :type Float%20%28double-precision%29))
  (return (* (Math|Trig|Sin(Degrees) (+ (* (Utilities|Time|GetGameTimeinSeconds) 3.6e+02) Offset)) 4e+01)))