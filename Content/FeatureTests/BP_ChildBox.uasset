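; BP_ChildBox is a feature-test actor that physically links its cube mesh to another Parent actor through a PhysicsControl component.
; On BeginPlay it casts the Parent's root to a static mesh component and creates a control between that and its own cube using ControlData.
; The control target is the box's starting transform relative to the Parent, so the control drives toward that initial offset and orientation.
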(event EventBeginPlay
  (bind _returnvalue (Transformation|GetActorTransform))
  (bind _parent (Variables|Default|GetParent))
  (bind _returnvalue_2 (Transformation|GetActorTransform _parent))
  (bind _returnvalue_3 (Math|Transform|MakeRelativeTransform _returnvalue _returnvalue_2))
  (bind _asstatic_mesh_component (Utilities|Casting|CastToStaticMeshComponent (Variables|/Script/Engine.Actor|GetRootComponent (Variables|Default|GetParent))))
  (Class|PhysicsControlComponent|MakeControl :self (Variables|Default|GetPhysicsControl) :ParentMeshComponent _asstatic_mesh_component :ChildMeshComponent (Variables|Default|GetCubeMesh) :ControlData (Variables|Default|GetControlData) :ControlTarget (Utilities|Struct|MakePhysicsControlTarget (.location _returnvalue_3) "0.000000,0.000000,0.000000" (.rotation _returnvalue_3))))

(event Collision|EventActorBeginOverlap
  (params (OtherActor :type Actor%20Object%20Reference)))

(event EventTick
  (params (DeltaSeconds :type Float%20%28single-precision%29)))

(fn ConstructionScript)