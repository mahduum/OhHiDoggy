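; Gameplay ability for a 90-degree turn in place, filed under canine abilities.
; On activation it switches the avatar mesh's root motion to everything and turns off controller rotation yaw on the avatar's instigator pawn.
; It then waits for a TurnInPlaceCompleted gameplay event to end itself.
; The logic restoring montage-only root motion and controller yaw is unconnected, so both changes persist after the ability ends.
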(event Ability|EventActivateAbility
  (bind _returnvalue (Ability|GetAvatarActorfromActorInfo))
  (Development|PrintString "Turn in place activated.")
  (Class|AnimInstance|SetRootMotionMode (Components|SkeletalMesh|GetAnimInstance (Actor|GetComponentbyClass _returnvalue "/Script/Engine.SkeletalMeshComponent")) "RootMotionFromEverything")
  (Variables|/Script/Engine.Pawn|SetbUseControllerRotationYaw (Variables|/Script/Engine.Actor|GetInstigator _returnvalue) false)
  (Ability|Tasks|WaitGameplayEvent "(TagName=\"TurnInPlaceCompleted\")" 0 true
    (:EventReceived
      (Ability|EndAbility))))

(event Ability|EventOnEndAbility
  (params (bWasCancelled :type Boolean))
  (Development|PrintString "Ability Ended"))

(event Ability|EventActivateAbilityFromEvent
  (params (EventData :type Gameplay%20Event%20Data%20Structure%20%28by%20ref%29)))