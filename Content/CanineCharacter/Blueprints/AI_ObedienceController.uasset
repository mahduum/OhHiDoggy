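; AI controller for the canine character that makes it follow a target, by default the first actor tagged "Echo".
; Custom events start following a given actor or stop it.
; On Tick, beyond the follow radius it moves directly without pathfinding, deriving walk speed from target speed and distance, with zero speed on sharp turns.
; Within the radius, it smoothly rotates in place toward the target.
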(event Custom|CustomEvent
  (params (Where :type Actor%20Object%20Reference))
  (Variables|Default|SetbFollow true)
  (Variables|Default|SetEcho Where))

(event Custom|CustomEvent_1
  (Variables|Default|SetbFollow false))

(event EventBeginPlay
  (bind _outactors (Actor|GetAllActorswithTag "Echo"))
  (if (Utilities|Array|IsValidIndex _outactors)
    (bind _output_get (Variables|Default|SetEcho (Utilities|Array|Get(acopy) _outactors)))
    (Variables|Default|SetLastForwardVector (Transformation|GetActorForwardVector _output_get))))

(event EventTick
  (params (DeltaSeconds :type Float%20%28single-precision%29))
  (bind _returnvalue (Pawn|GetControlledPawn))
  (bind _returnvalue_2 (Pawn|GetControlledPawn))
  (bind _returnvalue_3 (Pawn|GetDesiredRotation))
  (bind _echo (Variables|Default|GetEcho))
  (bind _slowdownthreshold (Variables|Default|GetSlowDownThreshold))
  (bind _echo_2 (Variables|Default|GetEcho))
  (bind _returnvalue_4 (Transformation|GetVelocity _echo_2))
  (bind _returnvalue_5 (Transformation|GetActorRotation _returnvalue))
  (bind _returnvalue_6 (Transformation|GetActorLocation _returnvalue_2))
  (bind _returnvalue_7 (Transformation|GetActorLocation _echo))
  (bind _returnvalue_8 (Actor|GetComponentbyClass _returnvalue_2 "/Script/Engine.CharacterMovementComponent"))
  (bind _returnvalue_9 (Math|Rotator|Delta(Rotator) _returnvalue_5 _returnvalue_3))
  (bind _returnvalue_10 (Math|Vector|Distance2D(Vector) _returnvalue_7 _returnvalue_6))
  (bind _returnvalue_11 (Math|Float|Absolute(Float) (.yaw _returnvalue_9)))
  (bind _returnvalue_12 (|ChaseOrFollowSpeed_2 _returnvalue_4 _returnvalue_10 _slowdownthreshold))
  (bind _returnvalue_13 (>= _returnvalue_11 9e+01))
  (if (and (Variables|Default|GetbFollow) (Utilities|IsValid _echo))
    (if (> _returnvalue_10 (Variables|Default|GetFollowRadius)) ; TODO: consider first turning towards target. If false just rotate.
      (bind _output_get (Variables|/Script/Engine.CharacterMovementComponent|SetMaxWalkSpeed _returnvalue_8 (select _returnvalue_13 0.0 (|SlowDownOrStop_2 _returnvalue_12 _returnvalue_12 _returnvalue_10)))) ; TODO: if Echo is still moving but the distance to her is less than\nacceptance radius minus some amount then start decreasing the\nspeed until the distance is again acceptance radius minus some other amount.
      (AI|Navigation|MovetoActor (Variables|Default|GetEcho) (Variables|Default|GetAcceptanceRadius) false false false 0) ; Hold on if it's turning sharply, maybe by setting speed to 0?
      (Variables|/Script/Engine.CharacterMovementComponent|SetbOrientRotationToMovement _returnvalue_8 (not _returnvalue_13)) ; TODO: Solve otherwise, do not rotate when root motion, but then include the new rotation from root motion.
      (else
        (|RotateInPlace_2 _returnvalue_2 _returnvalue_6 _returnvalue_7)))))

(fn ConstructionScript)